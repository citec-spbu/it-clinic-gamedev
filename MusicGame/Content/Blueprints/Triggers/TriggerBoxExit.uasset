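; Trigger box exit volume that brings up the main menu while the hero stands inside it.
; On hero overlap it resets the Blueprint_Hero's Health to 100, creates a W_MainMenu widget, adds it to the viewport and switches input to game-and-UI focused on it.
; When the hero leaves, it removes the widget from the screen.
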(event Collision|EventActorBeginOverlap
  (params (OtherActor :type Actor%20Object%20Reference))
  (bind _returnvalue (Game|GetPlayerController 0))
  (if (== (Utilities|GetClass OtherActor) "/Game/Blueprints/Hero/Blueprint_Hero.Blueprint_Hero_C")
    (bind _returnvalue_2 (Actor|GetActorOfClass "/Game/Blueprints/Hero/Blueprint_Hero.Blueprint_Hero_C"))
    (Variables|/Game/Blueprints/Hero/Blueprint_Hero.Blueprint_Hero_C|SetHealth _returnvalue_2 100)
    (bind _returnvalue_3 (UserInterface|CreateWidget "/Game/UI_MainMenu/W_MainMenu.W_MainMenu_C" _returnvalue))
    (bind _output_get (Variables|Default|SetWdgt _returnvalue_3))
    (UserInterface|Viewport|AddtoViewport _output_get 0)
    (Input|SetInputModeGameandUI _returnvalue _output_get "DoNotLock" true false)))

(event Collision|EventActorEndOverlap
  (params (OtherActor :type Actor%20Object%20Reference))
  (if (== (Utilities|GetClass OtherActor) "/Game/Blueprints/Hero/Blueprint_Hero.Blueprint_Hero_C")
    (Widget|RemovefromParent (Variables|Default|GetWdgt))))

(fn ConstructionScript)