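; One-shot trigger that spawns a second group of enemies when the hero walks into it.
; On overlap with an actor whose class is exactly Blueprint_Hero, it spawns Hogs and Hounds, then destroys itself.
; A shared SpawnActors function finds level actors by tag (HogSpawn2, HoundSpawn2) and spawns the given class at each one's transform.
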(event EventBeginPlay)

(event Collision|EventActorBeginOverlap
  (params (OtherActor :type Actor%20Object%20Reference))
  (if (== (Utilities|GetClass OtherActor) "/Game/Blueprints/Hero/Blueprint_Hero.Blueprint_Hero_C")
    (CallFunction|SpawnActors "HogSpawn2" "/Game/Blueprints/Enemies/Hog/Hog.Hog_C")
    (CallFunction|SpawnActors "HoundSpawn2" "/Game/Blueprints/Enemies/Hound/Hound.Hound_C")
    (Actor|DestroyActor)))

(event EventTick
  (params (DeltaSeconds :type Float%20%28single-precision%29)))

(fn ConstructionScript)

(fn SpawnActors
  (params (Tag :type String) (Class :type Actor%20Class%20Reference))
  (bind _outactors (Actor|GetAllActorswithTag (Utilities|String|StringToName Tag)))
  (for _array_element _outactors
    (Game|SpawnActorfromClass Class (Transformation|GetActorTransform _array_element) "Undefined" "MultiplyWithRoot" 0 0)))