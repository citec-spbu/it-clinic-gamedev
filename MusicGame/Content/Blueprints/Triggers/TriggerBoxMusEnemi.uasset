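; Trigger box actor that reacts to the hero entering and leaving its area, resetting hero stats and showing the W_MusEnemi widget.
; On overlap begin with Blueprint_Hero, it sets the hero's Health and Damage to fixed values, adds a new widget to the viewport and switches input to game-only.
; On overlap end, it removes the stored widget from the screen.
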(event EventBeginPlay)

(event Collision|EventActorBeginOverlap
  (params (OtherActor :type Actor%20Object%20Reference))
  (bind _returnvalue (Game|GetPlayerController 0))
  (if (== (Utilities|GetClass OtherActor) "/Game/Blueprints/Hero/Blueprint_Hero.Blueprint_Hero_C")
    (bind _returnvalue_2 (Actor|GetActorOfClass "/Game/Blueprints/Hero/Blueprint_Hero.Blueprint_Hero_C"))
    (Variables|/Game/Blueprints/Hero/Blueprint_Hero.Blueprint_Hero_C|SetHealth _returnvalue_2 100)
    (Variables|/Script/MusicGame.Hero_Base|Setdamage _returnvalue_2 5.0)
    (bind _returnvalue_3 (UserInterface|CreateWidget "/Game/UI_MainMenu/W_MusEnemi.W_MusEnemi_C" _returnvalue))
    (bind _output_get (Variables|Default|SetWdgt _returnvalue_3))
    (UserInterface|Viewport|AddtoViewport _output_get 0)
    (Input|SetInputModeGameOnly _returnvalue false)))

(event EventTick
  (params (DeltaSeconds :type Float%20%28single-precision%29)))

(event Collision|EventActorEndOverlap
  (params (OtherActor :type Actor%20Object%20Reference))
  (if (== (Utilities|GetClass OtherActor) "/Game/Blueprints/Hero/Blueprint_Hero.Blueprint_Hero_C")
    (Widget|RemovefromParent (Variables|Default|GetWdgt))))

(fn ConstructionScript)