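; TriggerBoxElMine is a trigger volume that restores the hero and shows the W_ElMine widget while the hero is inside.
; On overlap by an actor of exactly the Blueprint_Hero class, it sets the Health of the hero found through GetActorOfClass to a fixed value of 100.
; It then creates W_ElMine for player 0, stores it and adds it to the viewport, removing it when the hero leaves.
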(event EventBeginPlay)

(event Collision|EventActorBeginOverlap
  (params (OtherActor :type Actor%20Object%20Reference))
  (if (== (Utilities|GetClass OtherActor) "/Game/Blueprints/Hero/Blueprint_Hero.Blueprint_Hero_C")
    (bind _returnvalue (Actor|GetActorOfClass "/Game/Blueprints/Hero/Blueprint_Hero.Blueprint_Hero_C"))
    (Variables|/Game/Blueprints/Hero/Blueprint_Hero.Blueprint_Hero_C|SetHealth _returnvalue 100)
    (bind _returnvalue_2 (UserInterface|CreateWidget "/Game/UI_MainMenu/W_ElMine.W_ElMine_C" (Game|GetPlayerController 0)))
    (bind _output_get (Variables|Default|SetWdgt _returnvalue_2))
    (UserInterface|Viewport|AddtoViewport _output_get 0)))

(event EventTick
  (params (DeltaSeconds :type Float%20%28single-precision%29)))

(event Collision|EventActorEndOverlap
  (params (OtherActor :type Actor%20Object%20Reference))
  (if (== (Utilities|GetClass OtherActor) "/Game/Blueprints/Hero/Blueprint_Hero.Blueprint_Hero_C")
    (Widget|RemovefromParent (Variables|Default|GetWdgt))))

(fn ConstructionScript)