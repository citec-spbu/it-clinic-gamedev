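; BP_Sniper is a sprite-based enemy that fires on the hero, found at BeginPlay, whenever within horizontal attack range.
; Tick locks the player's position, shows a debug-drawn line trace as an aim telegraph, then spawns BP_SniperBullet toward that point after a short delay.
; Latent Delays in Tick pace subsequent shots.
; AnyDamage reduces health and jumps animation nodes to a brief damage stun, or to death followed by actor destruction.
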(event EventBeginPlay
  (bind _returnvalue (Actor|GetActorOfClass "/Game/Blueprints/Hero/Blueprint_Hero.Blueprint_Hero_C"))
  (Variables|Default|SetRefCharacter _returnvalue))

(event Collision|EventActorBeginOverlap
  (params (OtherActor :type Actor%20Object%20Reference)))

(event EventTick
  (params (DeltaSeconds :type Float%20%28single-precision%29))
  (bind _returnvalue (Transformation|GetActorLocation))
  (bind _sprite (Variables|Default|GetSprite))
  (bind _sprite_2 (Variables|Default|GetSprite))
  (bind _refcharacter (Variables|Default|GetRefCharacter))
  (bind _attackrange (Variables|Default|GetAttackRange))
  (bind _returnvalue_2 (Transformation|GetWorldTransform _sprite))
  (bind _returnvalue_3 (Transformation|GetWorldTransform _sprite_2))
  (bind _returnvalue_4 (Transformation|GetActorLocation _refcharacter))
  (bind _returnvalue_5 (- (.x (.location _returnvalue_3)) 4e+01))
  (bind _returnvalue_6 (- (.x _returnvalue_4) (.x _returnvalue)))
  (bind _returnvalue_7 (Math|Float|Absolute(Float) _returnvalue_6))
  (bind _returnvalue_8 (< _returnvalue_7 _attackrange))
  (if (and _returnvalue_8 (and (not (Variables|Default|GetisDead)) (not (Variables|Default|GetisDamaged))))
    (Variables|Default|SetisAttacking _returnvalue_8)
    (Class|PaperZDAnimInstance|JumptoNode (Variables|/Script/PaperZD.PaperZDAnimationComponent|GetAnimInstance (Variables|Default|GetAnimationComponent)) "Attack" "None")
    (if (Variables|Default|GetisAlreadyShoot)
      (Utilities|FlowControl|Delay 4.5))
    (bind _output_get (Variables|Default|SetplayerPosBeforeShoot (Transformation|GetActorLocation (Variables|Default|GetRefCharacter))))
    (Collision|MultiLineTraceByChannel (Math|Vector|MakeVector (- (.x (.location _returnvalue_2)) 4e+01) (.y (.location _returnvalue_2)) (.z (.location _returnvalue_2))) _output_get "TraceTypeQuery2" true 0 "ForDuration" true "(R=0.349565,G=0.000000,B=0.000000,A=1.000000)" "(R=0.350000,G=0.000000,B=0.000000,A=1.000000)" 0.5)
    (Utilities|FlowControl|Delay 0.5)
    (if (not (Variables|Default|GetisDead))
      (Game|SpawnActorfromClass "/Game/Blueprints/Enemies/Sniper/BP_SniperBullet.BP_SniperBullet_C" (Math|Transform|MakeTransform (Math|Vector|MakeVector _returnvalue_5 (.y (.location _returnvalue_3)) (.z (.location _returnvalue_3))) (Math|Conversions|RotationFromXVector (Math|Vector|Normalize (Math|Vector|GetUnitDirection(Vector) (Math|Vector|MakeVector _returnvalue_5 (.y (.location _returnvalue_3)) (.z (.location _returnvalue_3))) (Variables|Default|GetplayerPosBeforeShoot)))) (.scale _returnvalue_3)) "Undefined" "MultiplyWithRoot" 0 0)
      (Variables|Default|SetisAlreadyShoot true)
      (Variables|Default|SetisAttacking false))
    (else
      (Variables|Default|SetisAttacking false))))

(event Game|Damage|EventAnyDamage
  (params (Damage :type Float%20%28single-precision%29) (DamageType :type Damage%20Type%20Object%20Reference) (InstigatedBy :type Controller%20Object%20Reference) (DamageCauser :type Actor%20Object%20Reference))
  (if (not (Variables|Default|GetisDead))
    (Variables|Default|SetHealth (Math|Float|Truncate (- (Variables|Default|GetHealth) Damage)))
    (Development|PrintString (Utilities|String|Append (Utilities|String|ToString(Integer) (Variables|Default|GetHealth)) "Sniper health: ") true true "(R=1.000000,G=0.015124,B=0.000000,A=1.000000)")
    (if (> (Variables|Default|GetHealth) 0)
      (Variables|Default|SetisDamaged true)
      (Variables|Default|SetisAttacking false)
      (Class|PaperZDAnimInstance|JumptoNode (Variables|/Script/PaperZD.PaperZDAnimationComponent|GetAnimInstance (Variables|Default|GetAnimationComponent)) "Idle" "None")
      (Class|PaperZDAnimInstance|JumptoNode (Variables|/Script/PaperZD.PaperZDAnimationComponent|GetAnimInstance (Variables|Default|GetAnimationComponent)) "Damage" "None")
      (Utilities|FlowControl|Delay 0.5)
      (Variables|Default|SetisDamaged false)
      (else
        (Variables|Default|SetisDead true)
        (Variables|Default|SetisAttacking false)
        (Class|PaperZDAnimInstance|JumptoNode (Variables|/Script/PaperZD.PaperZDAnimationComponent|GetAnimInstance (Variables|Default|GetAnimationComponent)) "Idle" "None")
        (Class|PaperZDAnimInstance|JumptoNode (Variables|/Script/PaperZD.PaperZDAnimationComponent|GetAnimInstance (Variables|Default|GetAnimationComponent)) "Death" "None")
        (Utilities|FlowControl|Delay 1.0)
        (Actor|DestroyActor)))))

(fn ConstructionScript)