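; GI_MGame, apparently the Game Instance, provides the music volume setting through LoadVolume and SetVolume, backed by an SG_Settings save object.
; Both use cached CurSettings, falling back to loading the "Settings" slot or creating a new object, with LoadVolume defaulting to full volume.
; New objects save to the misspelled "Settimgs" slot, so the "Settings" lookup never finds them.
; SetVolume changes to cached or loaded settings stay in memory, unsaved here.
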(fn LoadVolume
  (if (Utilities|IsValid (Variables|Default|GetCurSettings))
    (return (Variables|/Game/Blueprints/SG_Settings.SG_Settings_C|GetMusVolume (Variables|Default|GetCurSettings)))
    (else
      (bind _returnvalue (SaveGame|DoesSaveGameExist "Settings"))
      (if _returnvalue
        (bind _returnvalue_2 (SaveGame|LoadGamefromSlot "Settings"))
        (bind _assg_settings (Utilities|Casting|CastToSG_Settings _returnvalue_2))
        (Variables|Default|SetCurSettings _assg_settings)
        (return (Variables|/Game/Blueprints/SG_Settings.SG_Settings_C|GetMusVolume _assg_settings))
        (else
          (bind _returnvalue_3 (SaveGame|CreateSaveGameObject "/Game/Blueprints/SG_Settings.SG_Settings_C"))
          (Variables|/Game/Blueprints/SG_Settings.SG_Settings_C|SetMusVolume _returnvalue_3 1.0)
          (SaveGame|SaveGametoSlot _returnvalue_3 "Settimgs")
          (Variables|Default|SetCurSettings _returnvalue_3)
          (return 1.0))))))

(fn SetVolume
  (params (NewVolume :type Float%20%28double-precision%29))
  (if (Utilities|IsValid (Variables|Default|GetCurSettings))
    (Variables|/Game/Blueprints/SG_Settings.SG_Settings_C|SetMusVolume (Variables|Default|GetCurSettings) NewVolume)
    (else
      (bind _returnvalue (SaveGame|DoesSaveGameExist "Settings"))
      (if _returnvalue
        (bind _returnvalue_2 (SaveGame|LoadGamefromSlot "Settings"))
        (bind _assg_settings (Utilities|Casting|CastToSG_Settings _returnvalue_2))
        (Variables|/Game/Blueprints/SG_Settings.SG_Settings_C|SetMusVolume _assg_settings NewVolume)
        (Variables|Default|SetCurSettings _assg_settings)
        (else
          (bind _returnvalue_3 (SaveGame|CreateSaveGameObject "/Game/Blueprints/SG_Settings.SG_Settings_C"))
          (Variables|/Game/Blueprints/SG_Settings.SG_Settings_C|SetMusVolume _returnvalue_3 NewVolume)
          (SaveGame|SaveGametoSlot _returnvalue_3 "Settimgs")
          (Variables|Default|SetCurSettings _returnvalue_3))))))