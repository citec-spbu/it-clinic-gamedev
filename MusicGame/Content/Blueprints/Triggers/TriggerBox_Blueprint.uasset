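; Trigger volume that shows the W_HelloTraining widget while the hero is inside it.
; On overlap with an actor of exactly the Blueprint_Hero class, it creates the widget for player 0, stores it in Wdgt and removes it on exit.
; If IsNeedSpawnPause is set, entry also adds the pause button and dash cooldown widgets, then clears the flag so they spawn once and stay on screen.
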(event EventBeginPlay)

(event Collision|EventActorBeginOverlap
  (params (OtherActor :type Actor%20Object%20Reference))
  (bind _returnvalue (Game|GetPlayerController 0))
  (if (== (Utilities|GetClass OtherActor) "/Game/Blueprints/Hero/Blueprint_Hero.Blueprint_Hero_C")
    (bind _returnvalue_2 (UserInterface|CreateWidget "/Game/UI_MainMenu/W_HelloTraining.W_HelloTraining_C" (Game|GetPlayerController 0)))
    (bind _output_get (Variables|Default|Setwdgt _returnvalue_2))
    (UserInterface|Viewport|AddtoViewport _output_get 0)
    (if (Variables|Default|GetisNeedSpawnPause)
      (bind _returnvalue_3 (UserInterface|CreateWidget "/Game/UI_MainMenu/W_PauseButton.W_PauseButton_C" _returnvalue))
      (UserInterface|Viewport|AddtoViewport _returnvalue_3 0)
      (bind _returnvalue_4 (UserInterface|CreateWidget "/Game/UI_MainMenu/W_DashCooldown.W_DashCooldown_C" _returnvalue))
      (UserInterface|Viewport|AddtoViewport _returnvalue_4 0)
      (Variables|Default|SetisNeedSpawnPause false))))

(event EventTick
  (params (DeltaSeconds :type Float%20%28single-precision%29)))

(event Collision|EventActorEndOverlap
  (params (OtherActor :type Actor%20Object%20Reference))
  (if (== (Utilities|GetClass OtherActor) "/Game/Blueprints/Hero/Blueprint_Hero.Blueprint_Hero_C")
    (Widget|RemovefromParent (Variables|Default|Getwdgt))))

(fn ConstructionScript)