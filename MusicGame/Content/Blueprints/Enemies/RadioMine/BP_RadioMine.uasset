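; BP_RadioMine is an enemy mine that explodes when a bullet or the hero overlaps it.
; It caches the Blueprint_Hero reference on BeginPlay and, on hero contact, sets the hero's IsCanReinforced flag to false.
; The shared Destroy graph swaps the Paper2D flipbook to the boom animation, waits briefly, hides it and destroys the actor.
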(event EventBeginPlay
  (bind _returnvalue (Actor|GetActorOfClass "/Game/Blueprints/Hero/Blueprint_Hero.Blueprint_Hero_C"))
  (Variables|Default|SetRefCharacter _returnvalue))

(event Collision|EventActorBeginOverlap
  (params (OtherActor :type Actor%20Object%20Reference))
  (Utilities|Casting|CastToBP_Bullet OtherActor
    (:then
      (Utilities|Destroy))
    (:CastFailed
      (if (== OtherActor (Variables|Default|GetRefCharacter))
        (Variables|/Script/MusicGame.Hero_Base|SetIsCanReinforced (Variables|Default|GetRefCharacter) false)
        (Sprite|SetFlipbook (Variables|Default|GetPaperFlipbook) "/Game/Assets/RadioMine/Boom/FB_RADIOMINE_BOOM.FB_RADIOMINE_BOOM")
        (Utilities|Destroy)))))

(event EventTick
  (params (DeltaSeconds :type Float%20%28single-precision%29)))

(fn ConstructionScript)