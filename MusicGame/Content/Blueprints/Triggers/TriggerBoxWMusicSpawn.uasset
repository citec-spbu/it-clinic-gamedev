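; TriggerBoxWMusicSpawn is a trigger that adds the music and damage widgets to the screen when the hero enters it.
; At BeginPlay it finds and stores the Blueprint_Hero actor.
; On overlap by that hero, while IsNeedSpawn is set, it creates W_Musik and W_Damage for player 0, adds both to the viewport and clears the flag so they spawn only once.
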(event EventBeginPlay
  (bind _returnvalue (Actor|GetActorOfClass "/Game/Blueprints/Hero/Blueprint_Hero.Blueprint_Hero_C"))
  (Variables|Default|SetCharacter _returnvalue))

(event Collision|EventActorBeginOverlap
  (params (OtherActor :type Actor%20Object%20Reference))
  (if (and (== OtherActor (Variables|Default|GetCharacter)) (Variables|Default|GetisNeedSpawn))
    (bind _returnvalue (UserInterface|CreateWidget "/Game/UI_Musik/W_Musik.W_Musik_C" (Game|GetPlayerController 0)))
    (UserInterface|Viewport|AddtoViewport _returnvalue 0)
    (bind _returnvalue_2 (UserInterface|CreateWidget "/Game/UI_Musik/W_Damage.W_Damage_C" (Game|GetPlayerController 0)))
    (UserInterface|Viewport|AddtoViewport _returnvalue_2 0)
    (Variables|Default|SetisNeedSpawn false)))

(event EventTick
  (params (DeltaSeconds :type Float%20%28single-precision%29)))

(fn ConstructionScript)