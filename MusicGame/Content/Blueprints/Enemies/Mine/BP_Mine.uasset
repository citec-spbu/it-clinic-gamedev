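; Paper2D mine hazard that explodes when touched by the hero or hit by a bullet.
; BeginPlay caches the Blueprint_Hero actor, and overlapping that actor applies fixed damage before detonating.
; An overlapping BP_Bullet also detonates the mine, without applying damage.
; BoomAndDestroy switches the flipbook to the Boom animation, waits briefly, hides it and destroys the actor.
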(event EventBeginPlay
  (bind _returnvalue (Actor|GetActorOfClass "/Game/Blueprints/Hero/Blueprint_Hero.Blueprint_Hero_C"))
  (Variables|Default|SetRefCharacter _returnvalue))

(event Collision|EventActorBeginOverlap
  (params (OtherActor :type Actor%20Object%20Reference))
  (if (== OtherActor (Variables|Default|GetRefCharacter))
    (Utilities|FlowControl|Sequence
      (:then_0
        (Game|Damage|ApplyDamage (Variables|Default|GetRefCharacter) 4e+01 0 0))
      (:then_1
        (Utilities|BoomandDestroy)))
    (else
      (Utilities|Casting|CastToBP_Bullet OtherActor)
      (if true
        (Utilities|BoomandDestroy)))))

(event EventTick
  (params (DeltaSeconds :type Float%20%28single-precision%29)))

(fn ConstructionScript)