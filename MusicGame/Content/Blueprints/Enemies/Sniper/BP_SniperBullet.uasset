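; BP_SniperBullet is the sniper enemy's projectile, which damages the hero on overlap.
; On BeginPlay it caches the Blueprint_Hero actor as its only valid damage target.
; Overlapping the hero applies fixed damage, hides the bullet component, stops ProjectileMovement and destroys the actor.
; Overlapping anything else destroys it after a short delay without stopping it, and there is no lifetime limit in the graph.
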(event EventBeginPlay
  (bind _returnvalue (Actor|GetActorOfClass "/Game/Blueprints/Hero/Blueprint_Hero.Blueprint_Hero_C"))
  (Variables|Default|SetRefCharacter _returnvalue))

(event Collision|EventActorBeginOverlap
  (params (OtherActor :type Actor%20Object%20Reference))
  (bind _refcharacter (Variables|Default|GetRefCharacter))
  (if (== OtherActor _refcharacter)
    (Game|Damage|ApplyDamage _refcharacter 4e+01 0 0)
    (Rendering|SetVisibility (Variables|Default|GetFB_SniperBullet) false false)
    (Components|Movement|StopMovementImmediately (Variables|Default|GetProjectileMovement))
    (else
      (Utilities|FlowControl|Delay 5.0)))
  (Actor|DestroyActor))

(event EventTick
  (params (DeltaSeconds :type Float%20%28single-precision%29)))

(fn ConstructionScript)